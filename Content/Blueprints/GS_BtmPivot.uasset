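; Bottom-pivot staircase piece that swings its flight about yaw and retracts or reveals railings when either the top or bottom trigger is overlapped.
; Five timelines play together on overlap, driving the flight's rotation, two retracting rails' X positions, and two tucked rails' X and roll via MoveXAndRoll.
; Ending overlap on either trigger reverses all five timelines after a delay, with no check for remaining occupants.
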(event OnComponentBeginOverlap(triggerTop)
  (params (OverlappedComponent :type Primitive%20Component%20Object%20Reference) (OtherActor :type Actor%20Object%20Reference) (OtherComp :type Primitive%20Component%20Object%20Reference) (OtherBodyIndex :type Integer) (bFromSweep :type Boolean) (SweepResult :type Hit%20Result%20Structure%20%28by%20ref%29))
  (bind _railuptuck (Variables|Default|GetRailUpTuck))
  (bind _raildownretract (Variables|Default|GetRailDownRetract))
  (bind _railupretract (Variables|Default|GetRailUpRetract))
  (bind _raildowntuck (Variables|Default|GetRailDownTuck))
  (bind _returnvalue (Transformation|GetRelativeTransform _railupretract))
  (bind _returnvalue_2 (Transformation|GetRelativeTransform _raildownretract))
  (bind (_location _rotation _scale) (Math|Transform|BreakTransform _returnvalue))
  (bind (_location_2 _rotation_2 _scale_2) (Math|Transform|BreakTransform _returnvalue_2))
  (bind (_x _y _z) (Math|Vector|BreakVector _location))
  (bind (_x_2 _y_2 _z_2) (Math|Vector|BreakVector _location_2))
  (Utilities|FlowControl|Sequence
    (:then_0
      (bind _railtranslation (Timeline|RetractRail Play)
        (:Update
          (Transformation|SetRelativeTransform (Variables|Default|GetRailDownRetract) (Math|Transform|MakeTransform (Math|Vector|MakeVector _railtranslation _y_2 _z_2) _rotation_2 _scale_2) false false))))
    (:then_1
      (bind _flightrotationz (Timeline|SwingRight Play)
        (:Update
          (Transformation|SetRelativeRotation (Variables|Default|GetFlight) (Math|Rotator|MakeRotator 0.0 0.0 _flightrotationz) true false))))
    (:then_2
      (bind (_direction _revealrail _swingrail) (Timeline|TuckedDownRailTimeline Play)
        (:Update
          (Transformation|SetRelativeTransform _raildowntuck (Utilities|MoveXandRoll _revealrail _swingrail _raildowntuck) false false))))
    (:then_3
      (bind _railtranslation_2 (Timeline|RetractRailDelayed Play)
        (:Update
          (Transformation|SetRelativeTransform (Variables|Default|GetRailUpRetract) (Math|Transform|MakeTransform (Math|Vector|MakeVector _railtranslation_2 _y _z) _rotation _scale) false false))))
    (:then_4
      (bind (_direction_2 _revealrail_2 _swingrail_2) (Timeline|TuckedUpRailTimeline Play)
        (:Update
          (Transformation|SetRelativeTransform _railuptuck (Utilities|MoveXandRoll _revealrail_2 _swingrail_2 _railuptuck) false false))))))

(event OnComponentBeginOverlap(triggerBottom)
  (params (OverlappedComponent :type Primitive%20Component%20Object%20Reference) (OtherActor :type Actor%20Object%20Reference) (OtherComp :type Primitive%20Component%20Object%20Reference) (OtherBodyIndex :type Integer) (bFromSweep :type Boolean) (SweepResult :type Hit%20Result%20Structure%20%28by%20ref%29))
  (bind _railuptuck (Variables|Default|GetRailUpTuck))
  (bind _raildownretract (Variables|Default|GetRailDownRetract))
  (bind _railupretract (Variables|Default|GetRailUpRetract))
  (bind _raildowntuck (Variables|Default|GetRailDownTuck))
  (bind _returnvalue (Transformation|GetRelativeTransform _railupretract))
  (bind _returnvalue_2 (Transformation|GetRelativeTransform _raildownretract))
  (bind (_location _rotation _scale) (Math|Transform|BreakTransform _returnvalue))
  (bind (_location_2 _rotation_2 _scale_2) (Math|Transform|BreakTransform _returnvalue_2))
  (bind (_x _y _z) (Math|Vector|BreakVector _location))
  (bind (_x_2 _y_2 _z_2) (Math|Vector|BreakVector _location_2))
  (Utilities|FlowControl|Sequence
    (:then_0
      (bind _railtranslation (Timeline|RetractRail Play)
        (:Update
          (Transformation|SetRelativeTransform (Variables|Default|GetRailDownRetract) (Math|Transform|MakeTransform (Math|Vector|MakeVector _railtranslation _y_2 _z_2) _rotation_2 _scale_2) false false))))
    (:then_1
      (bind _flightrotationz (Timeline|SwingRight Play)
        (:Update
          (Transformation|SetRelativeRotation (Variables|Default|GetFlight) (Math|Rotator|MakeRotator 0.0 0.0 _flightrotationz) true false))))
    (:then_2
      (bind (_direction _revealrail _swingrail) (Timeline|TuckedDownRailTimeline Play)
        (:Update
          (Transformation|SetRelativeTransform _raildowntuck (Utilities|MoveXandRoll _revealrail _swingrail _raildowntuck) false false))))
    (:then_3
      (bind _railtranslation_2 (Timeline|RetractRailDelayed Play)
        (:Update
          (Transformation|SetRelativeTransform (Variables|Default|GetRailUpRetract) (Math|Transform|MakeTransform (Math|Vector|MakeVector _railtranslation_2 _y _z) _rotation _scale) false false))))
    (:then_4
      (bind (_direction_2 _revealrail_2 _swingrail_2) (Timeline|TuckedUpRailTimeline Play)
        (:Update
          (Transformation|SetRelativeTransform _railuptuck (Utilities|MoveXandRoll _revealrail_2 _swingrail_2 _railuptuck) false false))))))

(event OnComponentEndOverlap(triggerBottom)
  (params (OverlappedComponent :type Primitive%20Component%20Object%20Reference) (OtherActor :type Actor%20Object%20Reference) (OtherComp :type Primitive%20Component%20Object%20Reference) (OtherBodyIndex :type Integer))
  (bind _railuptuck (Variables|Default|GetRailUpTuck))
  (bind _raildownretract (Variables|Default|GetRailDownRetract))
  (bind _railupretract (Variables|Default|GetRailUpRetract))
  (bind _raildowntuck (Variables|Default|GetRailDownTuck))
  (bind _returnvalue (Transformation|GetRelativeTransform _railupretract))
  (bind _returnvalue_2 (Transformation|GetRelativeTransform _raildownretract))
  (bind (_location _rotation _scale) (Math|Transform|BreakTransform _returnvalue))
  (bind (_location_2 _rotation_2 _scale_2) (Math|Transform|BreakTransform _returnvalue_2))
  (bind (_x _y _z) (Math|Vector|BreakVector _location))
  (bind (_x_2 _y_2 _z_2) (Math|Vector|BreakVector _location_2))
  (Utilities|FlowControl|Delay 5.0)
  (Utilities|FlowControl|Sequence
    (:then_0
      (bind _flightrotationz (Timeline|SwingRight Reverse)
        (:Update
          (Transformation|SetRelativeRotation (Variables|Default|GetFlight) (Math|Rotator|MakeRotator 0.0 0.0 _flightrotationz) true false))))
    (:then_1
      (bind _railtranslation (Timeline|RetractRail Reverse)
        (:Update
          (Transformation|SetRelativeTransform (Variables|Default|GetRailDownRetract) (Math|Transform|MakeTransform (Math|Vector|MakeVector _railtranslation _y_2 _z_2) _rotation_2 _scale_2) false false))))
    (:then_2
      (bind (_direction _revealrail _swingrail) (Timeline|TuckedDownRailTimeline Reverse)
        (:Update
          (Transformation|SetRelativeTransform _raildowntuck (Utilities|MoveXandRoll _revealrail _swingrail _raildowntuck) false false))))
    (:then_3
      (bind _railtranslation_2 (Timeline|RetractRailDelayed Reverse)
        (:Update
          (Transformation|SetRelativeTransform (Variables|Default|GetRailUpRetract) (Math|Transform|MakeTransform (Math|Vector|MakeVector _railtranslation_2 _y _z) _rotation _scale) false false))))
    (:then_4
      (bind (_direction_2 _revealrail_2 _swingrail_2) (Timeline|TuckedUpRailTimeline Reverse)
        (:Update
          (Transformation|SetRelativeTransform _railuptuck (Utilities|MoveXandRoll _revealrail_2 _swingrail_2 _railuptuck) false false))))))

(event OnComponentEndOverlap(triggerTop)
  (params (OverlappedComponent :type Primitive%20Component%20Object%20Reference) (OtherActor :type Actor%20Object%20Reference) (OtherComp :type Primitive%20Component%20Object%20Reference) (OtherBodyIndex :type Integer))
  (bind _railuptuck (Variables|Default|GetRailUpTuck))
  (bind _raildownretract (Variables|Default|GetRailDownRetract))
  (bind _railupretract (Variables|Default|GetRailUpRetract))
  (bind _raildowntuck (Variables|Default|GetRailDownTuck))
  (bind _returnvalue (Transformation|GetRelativeTransform _railupretract))
  (bind _returnvalue_2 (Transformation|GetRelativeTransform _raildownretract))
  (bind (_location _rotation _scale) (Math|Transform|BreakTransform _returnvalue))
  (bind (_location_2 _rotation_2 _scale_2) (Math|Transform|BreakTransform _returnvalue_2))
  (bind (_x _y _z) (Math|Vector|BreakVector _location))
  (bind (_x_2 _y_2 _z_2) (Math|Vector|BreakVector _location_2))
  (Utilities|FlowControl|Delay 5.0)
  (Utilities|FlowControl|Sequence
    (:then_0
      (bind _flightrotationz (Timeline|SwingRight Reverse)
        (:Update
          (Transformation|SetRelativeRotation (Variables|Default|GetFlight) (Math|Rotator|MakeRotator 0.0 0.0 _flightrotationz) true false))))
    (:then_1
      (bind _railtranslation (Timeline|RetractRail Reverse)
        (:Update
          (Transformation|SetRelativeTransform (Variables|Default|GetRailDownRetract) (Math|Transform|MakeTransform (Math|Vector|MakeVector _railtranslation _y_2 _z_2) _rotation_2 _scale_2) false false))))
    (:then_2
      (bind (_direction _revealrail _swingrail) (Timeline|TuckedDownRailTimeline Reverse)
        (:Update
          (Transformation|SetRelativeTransform _raildowntuck (Utilities|MoveXandRoll _revealrail _swingrail _raildowntuck) false false))))
    (:then_3
      (bind _railtranslation_2 (Timeline|RetractRailDelayed Reverse)
        (:Update
          (Transformation|SetRelativeTransform (Variables|Default|GetRailUpRetract) (Math|Transform|MakeTransform (Math|Vector|MakeVector _railtranslation_2 _y _z) _rotation _scale) false false))))
    (:then_4
      (bind (_direction_2 _revealrail_2 _swingrail_2) (Timeline|TuckedUpRailTimeline Reverse)
        (:Update
          (Transformation|SetRelativeTransform _railuptuck (Utilities|MoveXandRoll _revealrail_2 _swingrail_2 _railuptuck) false false))))))

(fn ConstructionScript)