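; Pivoting piece, apparently a stair flight, that swings around in yaw and moves its up and down rails when either the top or bottom trigger is overlapped.
; Five timelines play in parallel, rotating the Plane and retracting or tucking each rail through helper functions that change only selected relative-transform channels.
; Ending overlap on either trigger reverses all timelines after a fixed delay, with no check that the other trigger is clear.
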(event OnComponentBeginOverlap(triggerTop)
  (params (OverlappedComponent :type Primitive%20Component%20Object%20Reference) (OtherActor :type Actor%20Object%20Reference) (OtherComp :type Primitive%20Component%20Object%20Reference) (OtherBodyIndex :type Integer) (bFromSweep :type Boolean) (SweepResult :type Hit%20Result%20Structure%20%28by%20ref%29))
  (bind _raildownretract (Variables|Default|GetRailDownRetract))
  (bind _railupretract (Variables|Default|GetRailUpRetract))
  (bind _raiuptuck (Variables|Default|GetRaiUpTuck))
  (bind _raildowntuck (Variables|Default|GetRailDownTuck))
  (Utilities|FlowControl|Sequence
    (:then_0
      (bind _railtranslation (Timeline|RetractDownRail Play)
        (:Update
          (Transformation|SetRelativeTransform _raildownretract (Utilities|RetractRail _railtranslation _raildownretract) false false))))
    (:then_1
      (bind _flightrotationz (Timeline|Timeline_5 Play)
        (:Update
          (Transformation|SetRelativeRotation (Variables|Default|GetPlane) (Math|Rotator|MakeRotator 0.0 0.0 _flightrotationz) false false))))
    (:then_2
      (bind (_direction _revealrail _swingrail) (Timeline|TuckDownRail Play)
        (:Update
          (Transformation|SetRelativeTransform _raildowntuck (Utilities|MoveXandRoll _revealrail _swingrail _raildowntuck) false false))))
    (:then_3
      (bind _railtranslation_2 (Timeline|RetractUpRail Play)
        (:Update
          (Transformation|SetRelativeTransform _railupretract (Utilities|RetractRail _railtranslation_2 _railupretract) false false))))
    (:then_4
      (bind (_direction_2 _revealrailx _swingrail_2 _revealrailz) (Timeline|TuckUpRail Play)
        (:Update
          (Transformation|SetRelativeTransform _raiuptuck (Utilities|MoveandRoll _revealrailx _revealrailz _swingrail_2 _raiuptuck) false false))))))

(event OnComponentBeginOverlap(triggerBottom)
  (params (OverlappedComponent :type Primitive%20Component%20Object%20Reference) (OtherActor :type Actor%20Object%20Reference) (OtherComp :type Primitive%20Component%20Object%20Reference) (OtherBodyIndex :type Integer) (bFromSweep :type Boolean) (SweepResult :type Hit%20Result%20Structure%20%28by%20ref%29))
  (bind _raildownretract (Variables|Default|GetRailDownRetract))
  (bind _railupretract (Variables|Default|GetRailUpRetract))
  (bind _raiuptuck (Variables|Default|GetRaiUpTuck))
  (bind _raildowntuck (Variables|Default|GetRailDownTuck))
  (Utilities|FlowControl|Sequence
    (:then_0
      (bind _railtranslation (Timeline|RetractDownRail Play)
        (:Update
          (Transformation|SetRelativeTransform _raildownretract (Utilities|RetractRail _railtranslation _raildownretract) false false))))
    (:then_1
      (bind _flightrotationz (Timeline|Timeline_5 Play)
        (:Update
          (Transformation|SetRelativeRotation (Variables|Default|GetPlane) (Math|Rotator|MakeRotator 0.0 0.0 _flightrotationz) false false))))
    (:then_2
      (bind (_direction _revealrail _swingrail) (Timeline|TuckDownRail Play)
        (:Update
          (Transformation|SetRelativeTransform _raildowntuck (Utilities|MoveXandRoll _revealrail _swingrail _raildowntuck) false false))))
    (:then_3
      (bind _railtranslation_2 (Timeline|RetractUpRail Play)
        (:Update
          (Transformation|SetRelativeTransform _railupretract (Utilities|RetractRail _railtranslation_2 _railupretract) false false))))
    (:then_4
      (bind (_direction_2 _revealrailx _swingrail_2 _revealrailz) (Timeline|TuckUpRail Play)
        (:Update
          (Transformation|SetRelativeTransform _raiuptuck (Utilities|MoveandRoll _revealrailx _revealrailz _swingrail_2 _raiuptuck) false false))))))

(event OnComponentEndOverlap(triggerBottom)
  (params (OverlappedComponent :type Primitive%20Component%20Object%20Reference) (OtherActor :type Actor%20Object%20Reference) (OtherComp :type Primitive%20Component%20Object%20Reference) (OtherBodyIndex :type Integer))
  (bind _raildownretract (Variables|Default|GetRailDownRetract))
  (bind _railupretract (Variables|Default|GetRailUpRetract))
  (bind _raiuptuck (Variables|Default|GetRaiUpTuck))
  (bind _raildowntuck (Variables|Default|GetRailDownTuck))
  (Utilities|FlowControl|Delay 5.0)
  (Utilities|FlowControl|Sequence
    (:then_0
      (bind _flightrotationz (Timeline|Timeline_5 Reverse)
        (:Update
          (Transformation|SetRelativeRotation (Variables|Default|GetPlane) (Math|Rotator|MakeRotator 0.0 0.0 _flightrotationz) false false))))
    (:then_1
      (bind _railtranslation (Timeline|RetractDownRail Reverse)
        (:Update
          (Transformation|SetRelativeTransform _raildownretract (Utilities|RetractRail _railtranslation _raildownretract) false false))))
    (:then_2
      (bind (_direction _revealrail _swingrail) (Timeline|TuckDownRail Reverse)
        (:Update
          (Transformation|SetRelativeTransform _raildowntuck (Utilities|MoveXandRoll _revealrail _swingrail _raildowntuck) false false))))
    (:then_3
      (bind _railtranslation_2 (Timeline|RetractUpRail Reverse)
        (:Update
          (Transformation|SetRelativeTransform _railupretract (Utilities|RetractRail _railtranslation_2 _railupretract) false false))))
    (:then_4
      (bind (_direction_2 _revealrailx _swingrail_2 _revealrailz) (Timeline|TuckUpRail Reverse)
        (:Update
          (Transformation|SetRelativeTransform _raiuptuck (Utilities|MoveandRoll _revealrailx _revealrailz _swingrail_2 _raiuptuck) false false))))))

(event OnComponentEndOverlap(triggerTop)
  (params (OverlappedComponent :type Primitive%20Component%20Object%20Reference) (OtherActor :type Actor%20Object%20Reference) (OtherComp :type Primitive%20Component%20Object%20Reference) (OtherBodyIndex :type Integer))
  (bind _raildownretract (Variables|Default|GetRailDownRetract))
  (bind _railupretract (Variables|Default|GetRailUpRetract))
  (bind _raiuptuck (Variables|Default|GetRaiUpTuck))
  (bind _raildowntuck (Variables|Default|GetRailDownTuck))
  (Utilities|FlowControl|Delay 5.0)
  (Utilities|FlowControl|Sequence
    (:then_0
      (bind _flightrotationz (Timeline|Timeline_5 Reverse)
        (:Update
          (Transformation|SetRelativeRotation (Variables|Default|GetPlane) (Math|Rotator|MakeRotator 0.0 0.0 _flightrotationz) false false))))
    (:then_1
      (bind _railtranslation (Timeline|RetractDownRail Reverse)
        (:Update
          (Transformation|SetRelativeTransform _raildownretract (Utilities|RetractRail _railtranslation _raildownretract) false false))))
    (:then_2
      (bind (_direction _revealrail _swingrail) (Timeline|TuckDownRail Reverse)
        (:Update
          (Transformation|SetRelativeTransform _raildowntuck (Utilities|MoveXandRoll _revealrail _swingrail _raildowntuck) false false))))
    (:then_3
      (bind _railtranslation_2 (Timeline|RetractUpRail Reverse)
        (:Update
          (Transformation|SetRelativeTransform _railupretract (Utilities|RetractRail _railtranslation_2 _railupretract) false false))))
    (:then_4
      (bind (_direction_2 _revealrailx _swingrail_2 _revealrailz) (Timeline|TuckUpRail Reverse)
        (:Update
          (Transformation|SetRelativeTransform _raiuptuck (Utilities|MoveandRoll _revealrailx _revealrailz _swingrail_2 _raiuptuck) false false))))))

(fn ConstructionScript)